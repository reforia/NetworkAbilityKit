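; Behavior tree service that picks a movement location and target for an AI dragon each time it activates.
; In combat, it finds the closest of the dragon's targets and writes that actor, a random navigable location from it and a distance to the blackboard.
; Out of combat, it sets a random navigable location from the dragon itself and stores the dragon's distance from the world origin.
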(event EventReceiveActivationAI
  (params (OwnerController :type AI%20Controller%20Object%20Reference) (ControlledPawn :type Pawn%20Object%20Reference))
  (bind _targetlocation (Variables|Default|GetTargetLocation))
  (Variables|Default|SetMinDist 1e+05)
  (bind _asai_dragon (Utilities|Casting|CastToAI_Dragon ControlledPawn))
  (Variables|Default|SetDragonRef _asai_dragon)
  (if (Class|BTFunctionLibrary|GetBlackboardValueasBool (Variables|Default|GetInCombat))
    (for _array_element (Variables|/Game/ActionGame/Blueprint/AI_Dragon.AI_Dragon_C|GetTargets (Variables|Default|GetDragonRef))
      (if (< (Math|Vector|Distance(Vector) (Transformation|GetActorLocation _array_element) (Transformation|GetActorLocation (Variables|Default|GetDragonRef))) (Variables|Default|GetMinDist))
        (Variables|Default|SetMinDist (Math|Vector|Distance(Vector) (Transformation|GetActorLocation _array_element) (Transformation|GetActorLocation (Variables|Default|GetDragonRef))))
        (Variables|Default|SetClosestTarget _array_element)))
    (AI|BehaviorTree|SetBlackboardValueasVector _targetlocation (Default|GetRandomLocationonNav (Variables|Default|GetDragonRef) (Variables|Default|GetClosestTarget)))
    (Class|BTFunctionLibrary|SetBlackboardValueasObject (Variables|Default|GetTarget) (Variables|Default|GetClosestTarget))
    (Class|BTFunctionLibrary|SetBlackboardValueasFloat (Variables|Default|GetDistToTarget) (Math|Vector|Distance(Vector) (Default|GetRandomLocationonNav (Variables|Default|GetDragonRef) (Variables|Default|GetClosestTarget)) (Transformation|GetActorLocation (Variables|Default|GetDragonRef))))
    (else
      (AI|BehaviorTree|SetBlackboardValueasVector _targetlocation (Default|GetRandomLocationonNav (Variables|Default|GetDragonRef) (Variables|Default|GetDragonRef)))
      (Class|BTFunctionLibrary|SetBlackboardValueasFloat (Variables|Default|GetDistToTarget) (Math|Vector|Distance(Vector) (Transformation|GetActorLocation (Variables|Default|GetDragonRef)) "0, 0, 0")))))