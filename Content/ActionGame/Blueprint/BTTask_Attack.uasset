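; Behavior tree task that makes an AI_Dragon attack, choosing melee or non-melee by distance to target.
; It casts the pawn's anim instance to AnimBP_Dragon, sets melee when the DistToTarget blackboard value is under a fixed threshold, then sets the attack flag.
; It finishes successfully right away without waiting for the attack to play, and fails if either cast fails.
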(event EventReceiveExecuteAI
  (params (OwnerController :type AI%20Controller%20Object%20Reference) (ControlledPawn :type Pawn%20Object%20Reference))
  (bind _asai_dragon (Utilities|Casting|CastToAI_Dragon ControlledPawn)
    (:then
      (bind _asanim_bp_dragon (Utilities|Casting|CastToAnimBP_Dragon (Components|SkeletalMesh|GetAnimInstance (Variables|/Script/Engine.Character|GetMesh _asai_dragon)))
        (:then
          (Default|ServerSetMelee _asanim_bp_dragon (select (>= (Class|BTFunctionLibrary|GetBlackboardValueasFloat (Variables|Default|GetDistToTarget)) 7e+02) false true))
          (Default|ServerSetAttack _asanim_bp_dragon true)
          (AI|BehaviorTree|FinishExecute true))
        (:CastFailed
          (AI|BehaviorTree|FinishExecute false :!label _label))))
    (:CastFailed
      (goto _label))))