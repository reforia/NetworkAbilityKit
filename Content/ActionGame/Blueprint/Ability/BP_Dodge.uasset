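; BP_Dodge is an ability Blueprint that puts the controlled character into a dodging state.
; On activation it starts its cooldown, sets the InDodging stat on the controller's BPC_Action pawn, then ends immediately.
; The dodge movement and the clearing of that stat are not handled here.
; When the ability is unavailable, it prints the reason, such as cooldown, insufficient attributes or being disabled.
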(event EventBeginPlay
  (|CallParentFunction) ; This node is disabled and will not be called.\nDrag off pins to build functionality.
)

(event Collision|EventActorBeginOverlap
  (params (OtherActor :type Actor%20Object%20Reference))
  (|CallParentFunction OtherActor) ; This node is disabled and will not be called.\nDrag off pins to build functionality.
)

(event EventTick
  (params (DeltaSeconds :type Float%20%28single-precision%29))
  (|CallParentFunction DeltaSeconds) ; This node is disabled and will not be called.\nDrag off pins to build functionality.
)

(event EventOnActivated
  (Class|AbilityBase|StartCoolDown)
  (Utilities|FlowControl|Sequence
    (:then_0
      (bind _asbpc_action (Utilities|Casting|CastToBPC_Action (Pawn|GetControlledPawn (Variables|Default|GetBelongingController))))
      (CallFunction|TrySetStatsonTarget _asbpc_action "InDodging" true))
    (:then_1
      (Class|AbilityBase|EndAbility))))

(event EventOnCoolDownFinished)

(event EventOnNotAvailableYet
  (params (AbilityNotValidType :type EAbilityNotValidType%20Enum :default "ANV_DisabledInternally"))
  (Development|PrintString (Utilities|Select :Index AbilityNotValidType :ANV_DisabledInternally "I'm Not Available" :ANV_DisabledByModifier "I'm disabled by other modifiers" :ANV_InCoolDown "I'm in cooldown" :ANV_NotEnoughAttr "I don't have enough attributes" :ANV_PointUnavailable "The target point under mouse cursor is not Navable")))

(event EventOnAbilityPreEnd)

(fn ConstructionScript
  (|CallParentFunction))