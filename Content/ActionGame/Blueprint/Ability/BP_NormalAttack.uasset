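; Networked normal attack ability that plays a three-step twin-sword combo on a BPC_Action character.
; Activation starts the cooldown, toggles PlayMontage, calls the server combo event and ends the ability immediately.
; The server advances or resets ComboCount based on the pawn's NormalAttackCanCombo flag, then sets the matching montage with authority.
; Toggling PlayMontage acts as a replication trigger, with its OnRep playing the current Anim on the owner.
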(event Custom|SERVER_Combo
  (bind _asbpc_action (Utilities|Casting|CastToBPC_Action (Pawn|GetControlledPawn (Variables|Default|GetBelongingController))))
  (if (and (Variables|/Game/ActionGame/Blueprint/BPC_Action.BPC_Action_C|GetNormalAttackCanCombo _asbpc_action) (< (Variables|Default|GetComboCount) 2))
    (Math|Integer|IncrementInt (Variables|Default|GetComboCount)
      (:%20%20
        _))
    (else
      (Variables|Default|SetComboCount 0)))
  (CallFunction|SetAnimMontage (Utilities|Select :Index (Variables|Default|GetComboCount) :Option%200 "/Game/ActionGame/Animation/TwinSword_Attack_Start_1_Montage.TwinSword_Attack_Start_1_Montage" :Option%201 "/Game/ActionGame/Animation/TwinSword_Attack_Start_2_Montage.TwinSword_Attack_Start_2_Montage" :Option%202 "/Game/ActionGame/Animation/TwinSword_Attack17_Montage.TwinSword_Attack17_Montage")))

(event EventBeginPlay)

(event Collision|EventActorBeginOverlap
  (params (OtherActor :type Actor%20Object%20Reference)))

(event EventTick
  (params (DeltaSeconds :type Float%20%28single-precision%29)))

(event EventOnActivated
  (Class|AbilityBase|StartCoolDown)
  (Variables|Default|SetbPlayMontage (not (Variables|Default|GetbPlayMontage)))
  (Utilities|FlowControl|Sequence
    (:then_0
      (CallFunction|SERVERCombo))
    (:then_1
      (Class|AbilityBase|EndAbility))))

(event EventOnCoolDownFinished)

(event EventOnNotAvailableYet
  (params (AbilityNotValidType :type EAbilityNotValidType%20Enum :default "ANV_DisabledInternally"))
  (Development|PrintString (Utilities|Select :Index AbilityNotValidType :ANV_DisabledInternally "I'm Not Available" :ANV_DisabledByModifier "I'm disabled by other modifiers" :ANV_InCoolDown "I'm in cooldown" :ANV_NotEnoughAttr "I don't enough attributes" :ANV_PointUnavailable "The target point under mouse cursor is not Navable")))

(event EventOnAbilityPreEnd)

(fn ConstructionScript)

(fn SetAnimMontage
  (params (NewAnimMontage :type Anim%20Montage%20Object%20Reference))
  (Networking|SwitchHasAuthority
    (:Authority
      (Variables|Default|Setanim NewAnimMontage))))

(fn OnRepAnim)

(fn OnRepBPlayMontage
  (bind _asbpc_action (Utilities|Casting|CastToBPC_Action (Components|GetOwner)))
  (Animation|PlayAnimMontage _asbpc_action (Variables|Default|Getanim) 1.0 "None"))