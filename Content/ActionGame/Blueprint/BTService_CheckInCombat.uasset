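; Behavior tree service that maintains the InCombat blackboard flag for an AI_Dragon, cached on activation.
; Each tick with a valid Target, it loops over the dragon's Targets tracking MinDistanceToPlayers, but the combat range check uses the loop element's distance after the loop, not that minimum.
; Without a valid Target, InCombat follows whether TryGetTargetsInRange returns any targets.
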(event EventReceiveActivationAI
  (params (OwnerController :type AI%20Controller%20Object%20Reference) (ControlledPawn :type Pawn%20Object%20Reference))
  (bind _asai_dragon (Utilities|Casting|CastToAI_Dragon ControlledPawn))
  (Variables|Default|SetDragonRef _asai_dragon))

(event EventReceiveTickAI
  (params (OwnerController :type AI%20Controller%20Object%20Reference) (ControlledPawn :type Pawn%20Object%20Reference) (DeltaSeconds :type Float%20%28single-precision%29))
  (bind _dragonref (Variables|Default|GetDragonRef))
  (bind _incombat (Variables|Default|GetInCombat))
  (if (Utilities|IsValid (Class|BTFunctionLibrary|GetBlackboardValueasObject (Variables|Default|GetTarget)))
    (for _array_element (Variables|/Game/ActionGame/Blueprint/AI_Dragon.AI_Dragon_C|GetTargets _dragonref)
      (Variables|Default|SetMinDistanceToPlayers (Math|Float|Min(Float) (Math|Vector|Distance(Vector) (Transformation|GetActorLocation _array_element) (Transformation|GetActorLocation (Variables|Default|GetDragonRef))) (Variables|Default|GetMinDistanceToPlayers))))
    (if (< (Math|Vector|Distance(Vector) (Transformation|GetActorLocation _array_element) (Transformation|GetActorLocation (Variables|Default|GetDragonRef))) 1e+04)
      (Class|BTFunctionLibrary|SetBlackboardValueasBool _incombat true)
      (else
        (Class|BTFunctionLibrary|SetBlackboardValueasBool _incombat false)))
    (elif (> (Utilities|Array|Length (Default|TryGetTargetsinRange _dragonref)) 0)
      (Class|BTFunctionLibrary|SetBlackboardValueasBool _incombat true)
      (else
        (Class|BTFunctionLibrary|SetBlackboardValueasBool _incombat false)))))