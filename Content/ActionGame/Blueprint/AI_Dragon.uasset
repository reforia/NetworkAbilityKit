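; AI dragon enemy that tracks HP, shows it on floating text yawed toward the player, and damages non-dragon actors it touches.
; Front-foot and tail colliders deal random damage within a range, while multicast events set strafe, attack and melee states.
; Helper functions gather Player-tagged actors ahead within a sensing sphere, compute a signed turn angle to the target location, and pick random navmesh points in a cone toward a target.
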(event OnComponentBeginOverlap(FLFootCol)
  (params (OverlappedComponent :type Primitive%20Component%20Object%20Reference) (OtherActor :type Actor%20Object%20Reference) (OtherComp :type Primitive%20Component%20Object%20Reference) (OtherBodyIndex :type Integer) (bFromSweep :type Boolean) (SweepResult :type Hit%20Result%20Structure%20%28by%20ref%29))
  (CallFunction|ClientDealDamage OtherActor))

(event OnComponentBeginOverlap(FRFootCol)
  (params (OverlappedComponent :type Primitive%20Component%20Object%20Reference) (OtherActor :type Actor%20Object%20Reference) (OtherComp :type Primitive%20Component%20Object%20Reference) (OtherBodyIndex :type Integer) (bFromSweep :type Boolean) (SweepResult :type Hit%20Result%20Structure%20%28by%20ref%29))
  (CallFunction|ClientDealDamage OtherActor))

(event OnComponentBeginOverlap(Tail1Col)
  (params (OverlappedComponent :type Primitive%20Component%20Object%20Reference) (OtherActor :type Actor%20Object%20Reference) (OtherComp :type Primitive%20Component%20Object%20Reference) (OtherBodyIndex :type Integer) (bFromSweep :type Boolean) (SweepResult :type Hit%20Result%20Structure%20%28by%20ref%29))
  (CallFunction|ClientDealDamage OtherActor))

(event OnComponentBeginOverlap(Tail2Col)
  (params (OverlappedComponent :type Primitive%20Component%20Object%20Reference) (OtherActor :type Actor%20Object%20Reference) (OtherComp :type Primitive%20Component%20Object%20Reference) (OtherBodyIndex :type Integer) (bFromSweep :type Boolean) (SweepResult :type Hit%20Result%20Structure%20%28by%20ref%29))
  (CallFunction|ClientDealDamage OtherActor))

(event Custom|Multicast_SetMelee
  (params (Melee :type Boolean))
  (Variables|Default|SetMelee Melee))

(event Custom|Multicast_SetInStrafe
  (params (NewStrafe :type Boolean))
  (Variables|Default|SetInStrafe NewStrafe))

(event Custom|Multicast_SetAttacking
  (params (Attack :type Boolean))
  (Variables|Default|SetAttack Attack))

(event Custom|Client_DealDamage
  (params (Target :type Actor%20Object%20Reference))
  (Utilities|Casting|CastToAI_Dragon Target
    (:CastFailed
      (Game|Damage|ApplyDamage Target (Math|Random|RandomFloatinRange (Variables|Default|GetMinAttackDamage) (Variables|Default|GetMaxAttackDamage)) (Pawn|GetController) self))))

(event EventBeginPlay)

(event Collision|EventActorBeginOverlap
  (params (OtherActor :type Actor%20Object%20Reference)))

(event EventTick
  (params (DeltaSeconds :type Float%20%28single-precision%29))
  (bind _returnvalue (Game|GetPlayerCharacter 0))
  (Rendering|Components|TextRender|SetText (Variables|Default|GetTextRender) (Utilities|Text|ToText(Integer) (Math|Float|Floor (Variables|Default|GetHP))))
  (if (Utilities|IsValid _returnvalue)
    (Transformation|SetWorldRotation (Variables|Default|GetTextRender) (Math|Rotator|MakeRotator 0.0 0.0 (.yaw (Math|Rotator|FindLookatRotation (Transformation|GetActorLocation) (Transformation|GetActorLocation _returnvalue)))) false false)))

(event Game|Damage|EventAnyDamage
  (params (Damage :type Float%20%28single-precision%29) (DamageType :type Damage%20Type%20Object%20Reference) (InstigatedBy :type Controller%20Object%20Reference) (DamageCauser :type Actor%20Object%20Reference))
  (Variables|Default|SetHP (- (Variables|Default|GetHP) Damage)))

(fn ConstructionScript
  (Components|Sphere|SetSphereRadius (Variables|Default|GetVisualSensingZone) (Variables|Default|GetVisualSenseRange) true))

(fn TryGetTargetsinRange
  (Utilities|Array|Clear (Variables|Default|GetTargets))
  (for _array_element (Collision|GetOverlappingActors (Variables|Default|GetVisualSensingZone) "/Game/ActionGame/Blueprint/BPC_Action.BPC_Action_C" :!class /Script/Engine.PrimitiveComponent)
    (if (and (Utilities|Array|ContainsItem (Variables|/Script/Engine.Actor|GetTags _array_element) "Player") (> (Math|Vector|DotProduct (- (Transformation|GetActorLocation _array_element) (Transformation|GetActorLocation)) (Transformation|GetActorForwardVector)) 0.2))
      (Utilities|Array|AddUnique (Variables|Default|GetTargets) _array_element)))
  (return (Variables|Default|GetTargets)))

(fn GetDirectiontoTarget
  (bind _returnvalue (Transformation|GetActorLocation))
  (bind _returnvalue_2 (Transformation|GetActorForwardVector))
  (bind _targetlocation (Variables|Default|GetTargetLocation))
  (bind _returnvalue_3 (- _targetlocation _returnvalue))
  (bind _returnvalue_4 (Math|Vector|MakeVector (.x _returnvalue_2) (.y _returnvalue_2) 0.0))
  (bind _returnvalue_5 (Math|Vector|Normalize _returnvalue_4))
  (bind _returnvalue_6 (Math|Vector|Normalize _returnvalue_3))
  (bind (_x _y) (Math|Vector|BreakVector _returnvalue_6))
  (bind _returnvalue_7 (Math|Vector|MakeVector _x _y 0.0))
  (bind _returnvalue_8 (Math|Vector|Normalize _returnvalue_7))
  (if (> (Math|Vector|VectorLength _returnvalue_3) 1.0)
    (bind _output_get (Variables|Default|SetDirectionToTarget (* (Class|KismetMathLibrary|DegAcos (Math|Vector|DotProduct _returnvalue_8 _returnvalue_5)) (Math|Float|Sign(Float) (Math|Vector|DotProduct (Math|Vector|RotateVector _returnvalue_8 "0,-90.000000, 0") _returnvalue_5)))))
    (return _output_get)))

(fn GetRandomLocationonNav
  (params (AroundTarget :type Actor%20Object%20Reference))
  (bind _returnvalue (Transformation|GetActorLocation AroundTarget))
  (bind _returnvalue_2 (Transformation|GetActorLocation))
  (bind _returnvalue_3 (- _returnvalue _returnvalue_2))
  (bind _returnvalue_4 (Math|Vector|MakeVector (.x _returnvalue_3) (.y _returnvalue_3) 0.0))
  (bind _returnvalue_5 (Math|Vector|Normalize _returnvalue_4))
  (bind _returnvalue_6 (Math|Random|RandomUnitVectorinConeinDegrees _returnvalue_5 8e+01))
  (bind _output_get (Variables|Default|SetTargetLocation (.ProjectedLocation (AI|Navigation|ProjectPointtoNavigation (+ (Transformation|GetActorLocation AroundTarget) (* (Math|Vector|Normalize (Math|Vector|MakeVector (.x _returnvalue_6) (.y _returnvalue_6) 0.0)) (Math|Float|Min(Float) (Math|Vector|Distance(Vector) _returnvalue _returnvalue_2) (Math|Random|RandomFloatinRange (Variables|Default|GetMinDistance) (Variables|Default|GetMaxDistance))))) 0 0 "2000.000000,2000.000000,2000.000000"))))
  (return _output_get))