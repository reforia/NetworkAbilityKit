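; Game state for the Action mode that runs the pre-match countdown.
; A looping one-second timer checks each player state's initialization flag and counts down while all are ready.
; At zero it enables input on player controller 0 and clears the timer.
; CheckWinner and OnAllPlayerReady are empty; disconnected Arena logic would tally deaths by alternating-index teams and report wins or draws to the game mode.
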(event Custom|CheckPlayerInitializationState
  (bind _playerarray (Variables|Default|GetPlayerArray))
  (Variables|Default|SetPlayerFinishedInitializationCount 0)
  (for _array_element _playerarray
    (bind _asbpps_action (Utilities|Casting|CastToBPPS_Action _array_element))
    (if (Variables|/Game/ActionGame/Blueprint/BPPS_Action.BPPS_Action_C|GetPlayerFinishedInitialization _asbpps_action)
      (Math|Integer|IncrementInt (Variables|Default|GetPlayerFinishedInitializationCount))))
  (if (== (Variables|Default|GetPlayerFinishedInitializationCount) (Utilities|Array|Length _playerarray))
    (Variables|Default|SetAllPlayersReady true)
    (if (<= (Variables|Default|GetRemainingTimeToStart) 0.0)
      (Variables|Default|SetRemainingTimeToStart 0.0)
      (bind _asbp_action_controller (Utilities|Casting|CastToBP_ActionController (Game|GetPlayerController 0)))
      (Input|EnableInput _asbp_action_controller _asbp_action_controller)
      (Utilities|Time|ClearandInvalidateTimerbyHandle (Variables|Default|GetPreMatchTimerHandle))
      (else
        (Variables|Default|SetRemainingTimeToStart (- (Variables|Default|GetRemainingTimeToStart) 1.0))))))

(event Custom|CheckWinner)

(event Custom|OnAllPlayerReady)

(event EventBeginPlay
  (bind _returnvalue (Utilities|Time|SetTimerbyEvent (delegate Custom|CheckPlayerInitializationState) 1.0 true))
  (Variables|Default|SetPreMatchTimerHandle _returnvalue)
  (Variables|Default|SetRemainingTimeToStart (Variables|Default|GetTimeToStart)))

(event EventTick
  (params (DeltaSeconds :type Float%20%28single-precision%29)))

(fn ConstructionScript)