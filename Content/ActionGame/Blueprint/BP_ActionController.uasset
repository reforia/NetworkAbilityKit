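; Player controller for the networked action game that handles client setup, ability input and death.
; After login it disables input and creates the HUD.
; Post-initialization polls the pawn for ability, attribute and status sets with capped retries to fill the skill bar and bind death, flagging PlayerState finished after a delay.
; Attack and dodge inputs check status flags before requesting server activation; death notifies PlayerState, disables input and hides the pawn.
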(event Custom|FinishedInitialization
  ;[1 1 1] Finish Initialization
  (bind _asbpps_action (Utilities|Casting|CastToBPPS_Action (Variables|Default|GetPlayerState)))
  (Variables|/Game/ActionGame/Blueprint/BPPS_Action.BPPS_Action_C|SetPlayerFinishedInitialization _asbpps_action true))

(event Custom|AggresiveGetStatusSet
  ;[1 1 1] Get Status Set and Bind On Death Event
  (bind _asstat_set_action (Utilities|Casting|CastToStatSet_Action (Variables|/Script/NetworkAbilityKit.AttributeComp|GetStatusPreset (Actor|GetComponentbyClass (Pawn|GetControlledPawn) "/NetworkAbilityKit/Arena/NetworkAbility/Components/BPAC_Attribute.BPAC_Attribute_C")))
    (:then
      (Variables|Default|SetPawnStatusSet _asstat_set_action))
    (:CastFailed
      (Utilities|FlowControl|Delay 0.5)
      (bind _result (Math|Integer|IncrementInt (Variables|Default|GetClientGetStatusSetRetryAttempts))
        (:%20%20
          (if (>= _result 99)
            (Variables|Default|SetClientGetStatusSetRetryAttempts 0)
            (Development|PrintString "Client Get Status Set Failed!")
            (else
              (Development|PrintString (Utilities|String|Append "Attempt: " (Utilities|String|ToString(Integer) _result)))
              (CallFunction|AggresiveGetStatusSet))))))))

(event Custom|OnDeath
  ;[1 1 1] OnDeath Event
  (bind _asbpps_action (Utilities|Casting|CastToBPPS_Action (Variables|Default|GetPlayerState)))
  (Default|SERVERSetDeath _asbpps_action)
  (Input|DisableInput self)
  (Rendering|SetActorHiddenInGame (Pawn|GetControlledPawn) true))

(event Custom|AggresiveUpdateAbilityUI
  (bind _returnvalue (Pawn|GetControlledPawn))
  (bind (_abilitysetfind _abilityset) (CallFunction|GetActorAbilitySet _returnvalue))
  ;[1 1 1] Initialization
  (if _abilitysetfind
    (Variables|Default|SetPawnAbilitySet _abilityset)
    (Default|RefreshAbilityIcon (Variables|/Game/UI/UMG_MainAction_HUD.UMG_MainAction_HUD_C|GetUMG_Skill_Bar (Variables|Default|GetMainHUDRef)) (Variables|Default|GetPawnAbilitySet))
    (else
      (Utilities|FlowControl|Delay 0.5)
      (bind _result (Math|Integer|IncrementInt (Variables|Default|GetClientGetAbilitySetRetryAttempts))
        (:%20%20
          (if (>= _result 99)
            (Variables|Default|SetClientGetAbilitySetRetryAttempts 0)
            (Development|PrintString "Client UI Initialization Failed!")
            (else
              (Development|PrintString (Utilities|String|Append "Attempt: " (Utilities|String|ToString(Integer) _result)))
              (CallFunction|AggresiveUpdateAbilityUI))))))))

(event Custom|AggresiveGetAttributeSetAndBindDeathEvent
  ;[1 1 1] Get Attribute Set and Bind On Death Event
  (bind _asattr_set_action (Utilities|Casting|CastToAttrSet_Action (Variables|/Script/NetworkAbilityKit.AttributeComp|GetAttributePreset (Actor|GetComponentbyClass (Pawn|GetControlledPawn) "/NetworkAbilityKit/Arena/NetworkAbility/Components/BPAC_Attribute.BPAC_Attribute_C")))
    (:then
      (bind _output_get (Variables|Default|SetPawnAttributeSet _asattr_set_action))
      (EventDispatchers|BindEventtoOnDeathDelegate _output_get (delegate Custom|OnDeath)))
    (:CastFailed
      (Utilities|FlowControl|Delay 0.5)
      (bind _result (Math|Integer|IncrementInt (Variables|Default|GetClientGetAttributeSetRetryAttempts))
        (:%20%20
          (if (>= _result 99)
            (Variables|Default|SetClientGetAttributeSetRetryAttempts 0)
            (Development|PrintString "Client Get Attribute Set Failed!")
            (else
              (Development|PrintString (Utilities|String|Append "Attempt: " (Utilities|String|ToString(Integer) _result)))
              (CallFunction|AggresiveGetAttributeSetandBindDeathEvent))))))))

(event EventBeginPlay)

(event EventCLIENTPostLogin
  (bind _self self)
  ;[1 1 1] Initialization
  (Input|DisableInput self)
  (bind _returnvalue (UserInterface|CreateWidget "/Game/UI/UMG_MainAction_HUD.UMG_MainAction_HUD_C" _self))
  (if (Utilities|IsValid _returnvalue)
    (bind _output_get (Variables|Default|SetMainHUDRef _returnvalue))
    (UserInterface|Viewport|AddtoViewport _returnvalue 0)
    (Input|SetInputModeGameandUI _self _output_get "LockAlways" false)
    (Variables|/Script/Engine.PlayerController|SetbShowMouseCursor _self false)))

(event EventCLIENTPostInitialization
  ;[1 1 1] Initialization
  (CallFunction|AggresiveUpdateAbilityUI)
  (CallFunction|AggresiveGetAttributeSetandBindDeathEvent)
  (CallFunction|AggresiveGetStatusSet)
  (Utilities|FlowControl|Delay 2.0)
  (CallFunction|FinishedInitialization))

(event Input|ActionEvents|InputActionAction1
  (params (Key :type Key%20Structure :default "None"))
  (bind _self self)
  (bind _pawnstatusset (Variables|Default|GetPawnStatusSet))
  (bind (_abilityfind _ability) (CallFunction|FindLocalPlayerAbilitybyName _self "NormalAttack"))
  ;[1 1 1] Core Ability Call Section
  (:Pressed
    (if (and (.AttributeValue (Class|StatusSetBase|GetBoolAttribute _pawnstatusset "Equipped")) (not (.AttributeValue (Class|StatusSetBase|GetBoolAttribute _pawnstatusset "InAttacking"))))
      (if _abilityfind
        (Class|AbilityBehaviorCompBase|SERVERTryActivateAbility (Variables|Default|GetBPAC_AbilityBehavior) _ability)))))

(event Input|ActionEvents|InputActionAction3
  (params (Key :type Key%20Structure :default "None"))
  ;[1 1 1] Core Ability Call Section
)

(event Input|ActionEvents|InputActionAction2
  (params (Key :type Key%20Structure :default "None"))
  ;[1 1 1] Core Ability Call Section
)

(event Input|ActionEvents|InputActionAction4
  (params (Key :type Key%20Structure :default "None"))
  (bind _self self)
  (bind _pawnstatusset (Variables|Default|GetPawnStatusSet))
  (bind (_abilityfind _ability) (CallFunction|FindLocalPlayerAbilitybyName _self "Dodge"))
  (bind (_success _boolprop _attributevalue) (Class|StatusSetBase|GetBoolAttribute _pawnstatusset "InDodging"))
  ;[1 1 1] Core Ability Call Section
  (:Pressed
    (if (and _success (not _attributevalue))
      (if _abilityfind
        (Class|AbilityBehaviorCompBase|SERVERTryActivateAbility (Variables|Default|GetBPAC_AbilityBehavior) _ability)))))

(fn ConstructionScript)