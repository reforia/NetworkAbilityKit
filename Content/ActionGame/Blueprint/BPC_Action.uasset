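; Networked action character with dual-weapon melee, sprinting, jumping and target lock-on.
; Named stat flags gate input and drive per-tick updates of multicast walk speed and lock camera.
; Lock-on sphere-traces for a target, forces equipped state and aims the spring arm on non-authority instances.
; Multicast toggles weapon collision by attack state; overlaps damage actors other than BPC_Action, while received damage reduces attribute-set Health.
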(event OnComponentBeginOverlap(WLCollision)
  (params (OverlappedComponent :type Primitive%20Component%20Object%20Reference) (OtherActor :type Actor%20Object%20Reference) (OtherComp :type Primitive%20Component%20Object%20Reference) (OtherBodyIndex :type Integer) (bFromSweep :type Boolean) (SweepResult :type Hit%20Result%20Structure%20%28by%20ref%29))
  (CallFunction|CLIENTCallDealDamage OtherActor))

(event OnComponentBeginOverlap(WRCollision)
  (params (OverlappedComponent :type Primitive%20Component%20Object%20Reference) (OtherActor :type Actor%20Object%20Reference) (OtherComp :type Primitive%20Component%20Object%20Reference) (OtherBodyIndex :type Integer) (bFromSweep :type Boolean) (SweepResult :type Hit%20Result%20Structure%20%28by%20ref%29))
  (CallFunction|CLIENTCallDealDamage OtherActor))

(event Custom|SERVER_UpdateAttackCollision
  (CallFunction|MULTICASTUpdateAttackCollision))

(event Custom|MULTICAST_UpdateAttackCollision
  (if (.Value (CallFunction|TryGetStatsonTarget self "InAttacking"))
    (Collision|SetCollisionEnabled (Variables|Default|GetWLCollision) "QueryOnly")
    (Collision|SetCollisionEnabled (Variables|Default|GetWRCollision) "QueryOnly")
    (else
      (Collision|SetCollisionEnabled (Variables|Default|GetWLCollision) "NoCollision")
      (Collision|SetCollisionEnabled (Variables|Default|GetWRCollision) "NoCollision"))))

(event Custom|CLIENT_CallDealDamage
  (params (DamagedActor :type Actor%20Object%20Reference))
  (Utilities|Casting|CastToBPC_Action DamagedActor
    (:CastFailed
      (Game|Damage|ApplyDamage DamagedActor (Math|Random|RandomFloatinRange (Variables|Default|GetMinDmg) (Variables|Default|GetMaxDmg)) (Pawn|GetController) self "/NetworkAbilityKit/Arena/DamageType/BP_DmgType_Environment.BP_DmgType_Environment_C"))))

(event Custom|MULTICAST_SetMovementSpeed
  (params (NewSpeed :type Float%20%28single-precision%29))
  (Variables|/Script/Engine.CharacterMovementComponent|SetMaxWalkSpeed (Variables|Character|GetCharacterMovement) NewSpeed))

(event EventBeginPlay)

(event Collision|EventActorBeginOverlap
  (params (OtherActor :type Actor%20Object%20Reference)))

(event EventTick
  (params (DeltaSeconds :type Float%20%28single-precision%29))
  (CallFunction|UpdateSprintStatus)
  (CallFunction|UpdateSpeed)
  (CallFunction|UpdateLockMode)
  (Development|PrintString (Utilities|String|ToString(Float) (Variables|/Script/Engine.CharacterMovementComponent|GetMaxWalkSpeed (Variables|Character|GetCharacterMovement))) true true "(R=0.000000,G=0.660000,B=1.000000,A=1.000000)" 0.0))

(event EventMoveForward
  (params (AxisValue :type Float%20%28single-precision%29))
  (bind _self self)
  (bind _camcomp (Variables|Default|GetCamComp))
  (bind _value (CallFunction|TryGetStatsonTarget _self "InStopping"))
  (bind _returnvalue (Math|Vector|GetForwardVector _camcomp))
  (if (Math|Boolean|ANDBoolean (>= (Math|Float|Absolute(Float) AxisValue) 0.3) (not (.Value (CallFunction|TryGetStatsonTarget _self "InAttacking"))) (not _value))
    (Pawn|Input|AddMovementInput (Math|Vector|MakeVector (.x _returnvalue) (.y _returnvalue) 0.0) AxisValue false)
    (elif _value
      (Utilities|FlowControl|Delay 0.5)
      (CallFunction|TrySetStatsonTarget _self "InStopping" false))))

(event EventMoveRight
  (params (AxisValue :type Float%20%28single-precision%29))
  (bind _self self)
  (bind _camcomp (Variables|Default|GetCamComp))
  (bind _value (CallFunction|TryGetStatsonTarget _self "InStopping"))
  (bind _returnvalue (Math|Vector|GetRightVector _camcomp))
  (if (Math|Boolean|ANDBoolean (>= (Math|Float|Absolute(Float) AxisValue) 0.3) (not (.Value (CallFunction|TryGetStatsonTarget _self "InAttacking"))) (not _value))
    (Pawn|Input|AddMovementInput (Math|Vector|MakeVector (.x _returnvalue) (.y _returnvalue) 0.0) AxisValue false)
    (elif _value
      (Utilities|FlowControl|Delay 0.5)
      (CallFunction|TrySetStatsonTarget _self "InStopping" false))))

(event EventLookUp
  (params (AxisValue :type Float%20%28single-precision%29))
  (if (not (.Value (CallFunction|TryGetStatsonTarget self "InLockMode")))
    (Pawn|Input|AddControllerPitchInput AxisValue)))

(event EventLookRight
  (params (AxisValue :type Float%20%28single-precision%29))
  (if (not (.Value (CallFunction|TryGetStatsonTarget self "InLockMode")))
    (Pawn|Input|AddControllerYawInput AxisValue)))

(event Game|Damage|EventAnyDamage
  (params (Damage :type Float%20%28single-precision%29) (DamageType :type Damage%20Type%20Object%20Reference) (InstigatedBy :type Controller%20Object%20Reference) (DamageCauser :type Actor%20Object%20Reference))
  (bind _asbp_attr_set_action (Utilities|Casting|CastToBP_AttrSet_Action (Variables|/Script/NetworkAbilityKit.AttributeComp|GetAttributePreset (Variables|Default|GetBPAC_Attribute))))
  (Class|AttributeSetBase|SetFloatAttributeValuebyName _asbp_attr_set_action "Health" "AMM_Add" (* Damage -1.0))
  (Development|PrintString (Utilities|String|ToString(Float) (Variables|/Script/NetworkAbilityKit.AttrSet_Action|GetHealth _asbp_attr_set_action)) true true "(R=0.000000,G=0.047143,B=1.000000,A=1.000000)"))

(event Input|ActionEvents|InputActionEquip
  (params (Key :type Key%20Structure :default "None"))
  (bind _self self)
  (bind _self_2 self)
  (bind _value (CallFunction|TryGetStatsonTarget _self_2 "InEquipping"))
  (:Pressed
    (if (Math|Boolean|ANDBoolean (not _value) (not (.Value (CallFunction|TryGetStatsonTarget self "InDodging"))) (not (AI|Components|NavMovement|IsFalling (Variables|Character|GetCharacterMovement))))
      (CallFunction|ToggleEquipment)
      (elif _value
        (Utilities|FlowControl|Delay 2.0)
        (if (.Value (CallFunction|TryGetStatsonTarget _self "InEquipping"))
          (CallFunction|TrySetStatsonTarget _self "InEquipping" false))))))

(event Input|ActionEvents|InputActionJump
  (params (Key :type Key%20Structure :default "None"))
  (:Pressed
    (if (not (.Value (CallFunction|TryGetStatsonTarget self "InDodging")))
      (Character|Jump)))
  (:Released
    (Character|StopJumping)))

(event Input|ActionEvents|InputActionSprint
  (params (Key :type Key%20Structure :default "None"))
  (bind _self self)
  (:Pressed
    (CallFunction|TrySetStatsonTarget _self "InSprint" (not (.Value (CallFunction|TryGetStatsonTarget _self "InSprint"))))))

(event Input|ActionEvents|InputActionLock
  (params (Key :type Key%20Structure :default "None"))
  (:Pressed
    (CallFunction|ToggleLock)
    (if (.Value (CallFunction|TryGetStatsonTarget self "InLockMode"))
      (CallFunction|LockModeBehavior)
      (else
        (CallFunction|UnlockModeBehavior)))))

(fn ConstructionScript
  (CallFunction|MULTICASTSetMovementSpeed (Variables|Default|GetUnArmedRunSpeed)))

(fn ToggleEquipment
  (bind _self self)
  (CallFunction|TrySetStatsonTarget _self "Equipped" (not (.Value (CallFunction|TryGetStatsonTarget _self "Equipped")))))

(fn SetIsEquipping
  (params (NewEquippingState :type Boolean))
  (CallFunction|TrySetStatsonTarget self "InEquipping" NewEquippingState))

(fn ToggleLock
  (CallFunction|TrySetLock (not (.Value (CallFunction|TryGetStatsonTarget self "InLockMode")))))

(fn LockModeBehavior
  (CallFunction|SetEquipping true))

(fn UnlockModeBehavior)

(fn UpdateSprintStatus
  (if (and (== (Math|Vector|VectorLength (Transformation|GetVelocity)) 0.0) (.Value (CallFunction|TryGetStatsonTarget self "InSprint")))
    (CallFunction|TrySetStatsonTarget self "InSprint" false)))

(fn EquipWeapon
  (bind _mesh (Variables|Character|GetMesh))
  (bind _mesh_2 (Variables|Character|GetMesh))
  (if (.Value (CallFunction|TryGetStatsonTarget self "Equipped"))
    (Transformation|AttachComponentToComponent (Variables|Default|GetWeaponL) _mesh_2 "hand_lWeapon" "SnapToTarget" "SnapToTarget" "SnapToTarget" true)
    (Transformation|AttachComponentToComponent (Variables|Default|GetWeaponR) _mesh_2 "hand_rWeapon" "SnapToTarget" "SnapToTarget" "SnapToTarget" true)
    (else
      (Transformation|AttachComponentToComponent (Variables|Default|GetWeaponL) _mesh "spine_03lWeapon" "SnapToTarget" "SnapToTarget" "SnapToTarget" true)
      (Transformation|AttachComponentToComponent (Variables|Default|GetWeaponR) _mesh "spine_03rWeapon" "SnapToTarget" "SnapToTarget" "SnapToTarget" true))))

(fn SetEquipping
  (params (NewEquip :type Boolean))
  (CallFunction|TrySetStatsonTarget self "Equipped" NewEquip))

(fn TrySetLock
  (params (NewLock :type Boolean))
  (bind _array (Utilities|Array|MakeArray "ObjectTypeQuery7"))
  (bind _outactors (CallFunction|GetNearbyTargets _array))
  (if NewLock
    (if (> (Utilities|Array|Length _outactors) 0)
      (Variables|Default|SetLockedTarget (Utilities|Array|Get(acopy) _outactors))
      (CallFunction|TrySetStatsonTarget self "InLockMode" true)
      (else
        (CallFunction|TrySetStatsonTarget self "InLockMode" false :!label _label)
        (Variables|Default|SetLockedTarget 0)))
    (else
      (goto _label))))

(fn UpdateLockMode
  (bind _springarm (Variables|Default|GetSpringArm))
  (if (.Value (CallFunction|TryGetStatsonTarget self "InLockMode"))
    (Variables|/Script/Engine.SpringArmComponent|SetbUsePawnControlRotation _springarm false)
    (CallFunction|UpdateLockCamRotation)
    (else
      (Variables|/Script/Engine.SpringArmComponent|SetbUsePawnControlRotation _springarm true))))

(fn UpdateLockPlayerRotation
  (bind _camcomp (Variables|Default|GetCamComp))
  (bind _returnvalue (Math|Vector|GetForwardVector _camcomp))
  (Transformation|SetWorldRotation (Variables|Character|GetMesh) (Math|Rotator|CombineRotators (Math|Rotator|MakeRotfromX (Math|Vector|MakeVector (.x _returnvalue) (.y _returnvalue) 0.0)) "0,-90.000000, 0") false false))

(fn UpdateLockCamRotation
  (bind _mesh (Variables|Character|GetMesh))
  (bind _lockedtarget (Variables|Default|GetLockedTarget))
  (bind _returnvalue (Transformation|GetWorldLocation _mesh))
  (bind _returnvalue_2 (Transformation|GetActorLocation _lockedtarget))
  (bind _returnvalue_3 (Math|Rotator|FindLookatRotation _returnvalue _returnvalue_2))
  (Networking|SwitchHasAuthority
    (:Remote
      (if (Utilities|IsValid _lockedtarget)
        (Transformation|SetWorldRotation (Variables|Default|GetSpringArm) (Math|Rotator|MakeRotator 0.0 (.pitch _returnvalue_3) (.yaw _returnvalue_3)) false false)))))

(fn GetNearbyTargets
  (params (TargetTypes :type Array%20of%20EObjectTypeQuery%20Enums :default "ObjectTypeQuery1"))
  (bind _returnvalue (Transformation|GetActorLocation))
  (bind _outhits (Collision|MultiSphereTraceForObjects _returnvalue (+ _returnvalue "0.100000,0.100000,0.100000") (Variables|Default|GetLockingRange) TargetTypes false 0 "None"))
  (for _array_element _outhits
    (if (Utilities|IsValid (.HitActor (Collision|BreakHitResult _array_element)))
      (Utilities|Array|AddUnique (LocalVariables|GetTargetArray) (.HitActor (Collision|BreakHitResult _array_element)))))
  (return (LocalVariables|GetTargetArray)))

(fn UpdateAttackCollisionCheck
  (CallFunction|SERVERUpdateAttackCollision))

(fn UpdateSpeed
  (bind _self self)
  (bind _self_2 self)
  (bind _armedrunspeed (Variables|Default|GetArmedRunSpeed))
  (bind _armedsprintspeed (Variables|Default|GetArmedSprintSpeed))
  (bind _unarmedsprintspeed (Variables|Default|GetUnArmedSprintSpeed))
  (bind _unarmedrunspeed (Variables|Default|GetUnArmedRunSpeed))
  (bind _value (CallFunction|TryGetStatsonTarget _self_2 "InSprint"))
  (bind _value_2 (CallFunction|TryGetStatsonTarget _self "Equipped"))
  (bind _value_3 (CallFunction|TryGetStatsonTarget _self "Equipped"))
  (bind _returnvalue (select _value_3 _armedsprintspeed _unarmedsprintspeed))
  (bind _returnvalue_2 (select _value_2 _armedrunspeed _unarmedrunspeed))
  (bind _returnvalue_3 (select _value _returnvalue _returnvalue_2))
  (if (!= (Variables|/Script/Engine.CharacterMovementComponent|GetMaxWalkSpeed (Variables|Character|GetCharacterMovement)) _returnvalue_3)
    (CallFunction|MULTICASTSetMovementSpeed _returnvalue_3)))