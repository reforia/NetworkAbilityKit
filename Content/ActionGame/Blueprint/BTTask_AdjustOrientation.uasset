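; Behavior tree task that turns the AI dragon to face its TargetLocation before the tree continues.
; On execute it caches the controlled pawn as AI_Dragon, then each tick interpolates the actor's rotation toward the look-at rotation to that location.
; While turning it multicasts the strafe state on, and once the rotation is within a small tolerance it multicasts strafe off and finishes successfully.
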(event EventReceiveExecuteAI
  (params (OwnerController :type AI%20Controller%20Object%20Reference) (ControlledPawn :type Pawn%20Object%20Reference))
  (bind _asai_dragon (Utilities|Casting|CastToAI_Dragon ControlledPawn))
  (Variables|Default|SetDragonRef _asai_dragon))

(event EventReceiveTickAI
  (params (OwnerController :type AI%20Controller%20Object%20Reference) (ControlledPawn :type Pawn%20Object%20Reference) (DeltaSeconds :type Float%20%28single-precision%29))
  (bind _dragonref (Variables|Default|GetDragonRef))
  (bind _returnvalue (Transformation|GetActorRotation _dragonref))
  (bind _returnvalue_2 (Transformation|GetActorLocation _dragonref))
  (bind _targetlocation (Variables|/Game/ActionGame/Blueprint/AI_Dragon.AI_Dragon_C|GetTargetLocation _dragonref))
  (bind _returnvalue_3 (Math|Rotator|FindLookatRotation _returnvalue_2 _targetlocation))
  (Transformation|SetActorRotation _dragonref (Math|Interpolation|RInterpTo _returnvalue _returnvalue_3 DeltaSeconds 1e+01))
  (if (Math|Rotator|Equal(Rotator) _returnvalue _returnvalue_3 0.1)
    (Default|MulticastSetinStrafe _dragonref false)
    (AI|BehaviorTree|FinishExecute true)
    (else
      (Default|MulticastSetinStrafe _dragonref true))))